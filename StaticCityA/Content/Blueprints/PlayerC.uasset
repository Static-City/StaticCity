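; PlayerC is a player character Blueprint that handles basic movement, jumping and look input.
; MoveForward and MoveRight axes add movement along the actor's forward and right vectors, and Space Bar triggers Jump.
; The look axes feed controller rotation crosswise to their names: LookVertical drives yaw and LookHorizontal drives pitch.
; The movement graph is marked as needing a fix, and the construction script is empty.
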(event Input|AxisEvents|InputAxisMoveForward
  (params (AxisValue :type Float%20%28single-precision%29))
  ;[1 1 1] Movement(PLEASE FIX)
  (Pawn|Input|AddMovementInput (Transformation|GetActorForwardVector) AxisValue false))

(event Input|AxisEvents|InputAxisMoveRight
  (params (AxisValue :type Float%20%28single-precision%29))
  ;[1 1 1] Movement(PLEASE FIX)
  (Pawn|Input|AddMovementInput (Transformation|GetActorRightVector) AxisValue false))

(event Input|AxisEvents|InputAxisLookVertical
  (params (AxisValue :type Float%20%28single-precision%29))
  ;[1 1 1] Movement(PLEASE FIX)
  (Pawn|Input|AddControllerYawInput AxisValue))

(event Input|AxisEvents|InputAxisLookHorizontal
  (params (AxisValue :type Float%20%28single-precision%29))
  ;[1 1 1] Movement(PLEASE FIX)
  (Pawn|Input|AddControllerPitchInput AxisValue))

(event Input|KeyboardEvents|SpaceBar
  (params (Key :type Key%20Structure :default "None"))
  ;[1 1 1] Movement(PLEASE FIX)
  (:Pressed
    (Character|Jump)))

(fn ConstructionScript)